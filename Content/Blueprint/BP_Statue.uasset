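; Statue that emits a fire beam, stopping at whatever it hits or at maximum range.
; BeginPlay spawns a BP_Feu beam actor above the statue and a separate fire impact emitter.
; Each Tick, a Camera-channel line trace sets the beam's end, then moves the impact effect and BP_Feu's blocking hitbox just short of it.
; The construction script angles the Sphere, used as beam source and rotation reference, when FaceDown is set.
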(event `self.ReceiveTick`
  (params (DeltaSeconds :type "Float (single-precision)"))
  (bind _impact (`self.Impact`))
  (bind _fire (`self.FIRE`))
  (bind _returnvalue (`SceneComponent.K2_GetComponentRotation` (`self.Sphere`)))
  (bind _laser_target_point (`/Game/Blueprint/BP_Feu.laser target point` _fire))
  (bind _particle (`/Game/Blueprint/BP_Feu.Particle` _fire))
  (bind _particle_2 (`/Game/Blueprint/BP_Feu.Particle` (`self.FIRE`)))
  (bind _box (`/Game/Blueprint/BP_Feu.Box` _fire))
  (bind _returnvalue_2 (`SceneComponent.GetForwardVector` _particle_2))
  (bind _returnvalue_3 (`SceneComponent.K2_GetComponentLocation` _particle_2))
  (bind _returnvalue_4 (+ _returnvalue_3 (* _returnvalue_2 4000)))
  (bind (_outhit _returnvalue_5) (`KismetSystemLibrary.LineTraceSingle` _returnvalue_3 _returnvalue_4 "TraceTypeQuery2"))
  (if _returnvalue_5
    (set `self.HitActor` (`.HitActor` (`GameplayStatics.BreakHitResult` _outhit)))
    (set `/Game/Blueprint/BP_Feu.laser target point` (`.Location` (`GameplayStatics.BreakHitResult` _outhit)) _fire)
    (else
      (set `/Game/Blueprint/BP_Feu.laser target point` _returnvalue_4 _fire)))
  ;[1 0.8745 0.3569] Réglage de la longueur du laser
  (`ParticleSystemComponent.SetBeamSourcePoint` _particle 0 (`SceneComponent.K2_GetComponentLocation` (`self.Sphere`)) 0)
  (`ParticleSystemComponent.SetBeamTargetPoint` _particle 0 _laser_target_point 0)
  ;[1 0.8745 0.3569] Déplacement de l'emitter d'impact
  (`SceneComponent.K2_SetWorldLocation` _impact (- _laser_target_point (* _returnvalue_2 100)) false true)
  (`SceneComponent.K2_SetWorldRotation` _impact _returnvalue false false)
  ;[1 0.8745 0.3569] Déplacement de la hitbox de blocage
  (`SceneComponent.K2_SetWorldLocation` _box (- _laser_target_point (* _returnvalue_2 10)) false true)
  (`SceneComponent.K2_SetWorldRotation` _box _returnvalue true true))

(event `self.ReceiveActorBeginOverlap`
  (params (OtherActor :type "Actor Object Reference")))

(event `self.ReceiveBeginPlay`
  (bind _returnvalue (`|SpawnActorFromClass` "/Game/Blueprint/BP_Feu.BP_Feu_C" (`KismetMathLibrary.MakeTransform` (+ (`self.K2_GetActorLocation`) (0.0 0.0 120.0)) (`self.K2_GetActorRotation`) (1.0 1.0 1.0)) "AlwaysSpawn" "OverrideRootScale"))
  (set `self.FIRE` _returnvalue)
  (bind _returnvalue_2 (`GameplayStatics.SpawnEmitterAtLocation` "/Game/Effects/System_Particules/PS_Crache_Feu_Impact.PS_Crache_Feu_Impact"))
  (set `self.Impact` _returnvalue_2))

(fn `UserConstructionScript`
  (if (`self.FaceDown`)
    (`SceneComponent.K2_SetRelativeRotation` (`self.Sphere`) (struct :`Pitch` -10.0) false false)
    (else
      (`SceneComponent.K2_SetRelativeRotation` (`self.Sphere`) (struct) false false))))