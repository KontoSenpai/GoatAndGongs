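; Camera actor that becomes the view for player controller 0 when play begins.
; The construction script gives its camera component a fixed world rotation.
; Tick does nothing: the logic to follow the first BP_Joueur with an offset location and adjusted rotation is disconnected, so nothing here moves the camera during play.
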(event `self.ReceiveBeginPlay`
  (`PlayerController.SetViewTargetWithBlend` (`GameplayStatics.GetPlayerController` 0) self 0.0 "VTBlend_Linear" 0.0 false))

(event `self.ReceiveTick`
  (params (DeltaSeconds :type "Float (single-precision)")))

(fn `UserConstructionScript`
  (`SceneComponent.K2_SetWorldRotation` (`self.CameraComponent`) (struct :`Pitch` -60.0) false false))