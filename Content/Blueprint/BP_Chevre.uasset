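; Goat character that walks itself to the first NavigationTestingActor's location, retrying failed moves and completing the level on arrival.
; Touching BP_Feu kills it: it stops, gets a burn material, updates the goat score and reloads the level.
; Players overlapping its head hitbox are launched away every tick, with a timed PlayerFlying flag.
; Its construction script makes the capsule ignore two players when moving so they cannot block it.
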(event `self.ReceiveBeginPlay`
  ;[0.3619 0.6576 1] PathFinding
  (`KismetSystemLibrary.Delay` 1.0)
  (bind _outactors (`GameplayStatics.GetAllActorsOfClass` "/Game/Blueprint/BP_Joueur.BP_Joueur_C"))
  (for (_array_element _array_index) _outactors
    (`KismetArrayLibrary.Array_Set` (`self.tableau_joueurs`) _array_index _array_element true)
    (`KismetArrayLibrary.Array_Set` (`self.RepulsePlayer`) _array_index false true))
  (`KismetSystemLibrary.Delay` 0.5)
  (set `CharacterMovementComponent.MaxWalkSpeed` (`self.MvtSpeed`) (`self.CharacterMovement`))
  (bind _destination (`self.PathFinding` :!label _label))
  (`|AIMoveTo` self _destination
    (:`OnSuccess`
      (bind _outactors_2 (`GameplayStatics.GetAllActorsOfClass` "/Game/Blueprint/BP_Joueur.BP_Joueur_C"))
      (for _array_element_2 _outactors_2
        (set `/Game/Blueprint/BP_Joueur.EndLevelInvincibility` true _array_element_2)
        (set `/Game/Blueprint/BP_Joueur.Block` false _array_element_2))
      (bind _outactors_3 (`GameplayStatics.GetAllActorsOfClass` "/Game/Blueprint/MyGame.MyGame_C"))
      (`/Game/Blueprint/MyGame.LevelCompleteResetScore` (`KismetArrayLibrary.Array_Get` _outactors_3)))
    (:`OnFail`
      (if (`self.IsDead?_Goat`)
        (`MovementComponent.StopMovementImmediately` (`self.CharacterMovement`))
        (else
          (goto _label))))))

(event `self.HitBox Chèvre.OnComponentBeginOverlap`
  (params (OtherActor :type "Actor Object Reference") (OtherComp :type "PrimitiveComponent Object Reference") (OtherBodyIndex :type Integer) (bFromSweep :type Boolean) (SweepResult :type "HitResult Structure (by ref)"))
  ;[0.3922 1 0.6314] Death + retry
  (if (== (`GameplayStatics.GetObjectClass` OtherActor) "/Game/Blueprint/BP_Feu.BP_Feu_C")
    (set `self.IsDead?_Goat` true)
    (`|ExecutionSequence`
      (:`then_0`
        (bind _returnvalue (`PrimitiveComponent.CreateDynamicMaterialInstance` (`self.Mesh`) 0 "/Game/Materials/M_Lave.M_Lave"))
        (`KismetSystemLibrary.Delay` 0.3)
        (`MovementComponent.StopMovementImmediately` (`self.CharacterMovement`))
        (`MaterialInstanceDynamic.SetScalarParameterValue` _returnvalue "Opacité du Burn Value" 1.0)
        (`self.SetActorEnableCollision` false))
      (:`then_1`
        (bind _outactors (`GameplayStatics.GetAllActorsOfClass` "/Game/Blueprint/MyGame.MyGame_C"))
        (`/Game/Blueprint/MyGame.UpdateScoreGoat` (`KismetArrayLibrary.Array_Get` _outactors)))
      (:`then_2`
        (`KismetSystemLibrary.Delay` 2.0)
        (bind _returnvalue_2 (`GameplayStatics.GetCurrentLevelName` true))
        (`GameplayStatics.OpenLevel` (`KismetStringLibrary.Conv_StringToName` _returnvalue_2))))))

(event `self.Hitbox Tete.OnComponentBeginOverlap`
  (params (OtherActor :type "Actor Object Reference") (OtherComp :type "PrimitiveComponent Object Reference") (OtherBodyIndex :type Integer) (bFromSweep :type Boolean) (SweepResult :type "HitResult Structure (by ref)"))
  ;[1 1 1] Création des BP_Joueur dans tableau_joueurs qui overlappent avec la chèvre
  (if (== (`GameplayStatics.GetObjectClass` OtherActor) "/Game/Blueprint/BP_Joueur.BP_Joueur_C")
    (for (_array_element _array_index) (`self.tableau_joueurs`)
      (if (== _array_element OtherActor)
        (`KismetArrayLibrary.Array_Set` (`self.RepulsePlayer`) _array_index true)))))

(event `self.Hitbox Tete.OnComponentEndOverlap`
  (params (OtherActor :type "Actor Object Reference") (OtherComp :type "PrimitiveComponent Object Reference") (OtherBodyIndex :type Integer))
  ;[1 1 1] Ajouter les elements en overlap avec la chèvre
  (if (== (`GameplayStatics.GetObjectClass` OtherActor) "/Game/Blueprint/BP_Joueur.BP_Joueur_C")
    (for (_array_element _array_index) (`self.tableau_joueurs`)
      (if (== _array_element OtherActor)
        (`KismetArrayLibrary.Array_Set` (`self.RepulsePlayer`) _array_index false)))))

(event `self.ReceiveTick`
  (params (DeltaSeconds :type "Float (single-precision)"))
  ;[1 0 0.54] Lorsqu'on entre en contact avec le joueur ce dernier est propulsé
  (for (_array_element _array_index) (`self.tableau_joueurs`)
    (if (`KismetArrayLibrary.Array_Get` (`self.RepulsePlayer`) _array_index)
      (set `self.PlayerFlying` true)
      (`self.LaunchCharacter` _array_element (+ (* (`KismetMathLibrary.Normal` (- (`self.K2_GetActorLocation` _array_element) (`SceneComponent.K2_GetComponentLocation` (`self.Hitbox Tete`)))) (`self.ForceDuDeplacementJoueurChevre`)) (0.0 0.0 3.0)) false false)
      (set `self.AnimationTriggerTime` (`KismetMathLibrary.Now`))))
  (if (> (- (`KismetMathLibrary.GetTotalMilliseconds` (`KismetMathLibrary.GetTimeOfDay` (`KismetMathLibrary.Now`))) (`KismetMathLibrary.GetTotalMilliseconds` (`KismetMathLibrary.GetTimeOfDay` (`self.AnimationTriggerTime`)))) (`self.Animation duration`))
    (set `self.PlayerFlying` false)))

(fn `PathFinding`
  (returns (Destination :type "Vector Structure"))
  (`|ExecutionSequence`
    (:`then_1`
      (bind _outactors (`GameplayStatics.GetAllActorsOfClass` "/Script/Engine.NavigationTestingActor"))
      (bind _item (`KismetArrayLibrary.Array_Get` _outactors))
      (if (`KismetSystemLibrary.IsValid` _item)
        (return (`self.K2_GetActorLocation` _item))))))

(fn `UserConstructionScript`
  ;[1 0.9041 0.3456] Avoid being blocked by Players
  (bind _outactors (`GameplayStatics.GetAllActorsOfClass` "/Game/Blueprint/BP_Joueur.BP_Joueur_C"))
  (for _index (range 2)
    (`PrimitiveComponent.IgnoreActorWhenMoving` (`self.CapsuleComponent`) (`KismetArrayLibrary.Array_Get` _outactors _index) true)
    (set `self.ChevreSelf` self)))